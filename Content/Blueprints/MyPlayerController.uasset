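; Player controller that runs the core loop of a tile-based survival game about crossing city layers while fire advances.
; Tile moves lerp the character on Tick, spend distance-based fuel and food, then check win/lose and spread fire row by row after a grace period.
; Reaching a new layer rebuilds the random tile grid.
; Interacting with tiles grants resources with random setbacks, reported through the in-game log and timed notifications.
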(event Custom|MoveCharacter
  (Utilities|Casting|CastToMyPlayerController (Game|GetPlayerController 0))
  (Variables|Default|SetmoveProgress 0.0))

(event EventBeginPlay)

(event EventTick
  (params (DeltaSeconds :type Float%20%28single-precision%29))
  (CallFunction|UpdateMoveProgressifNeeded DeltaSeconds))

(event Input|ActionEvents|InputActionRestart
  (params (Key :type Key%20Structure))
  (:Pressed
    (Game|OpenLevel(byName) "Minimal_Default")))

(event Input|ActionEvents|InputActionGameOver
  (params (Key :type Key%20Structure))
  (:Pressed
    (Variables|Default|SetgameHullHP 0)
    (CallFunction|VerifyLoseCondition)))

(fn ConstructionScript)

(fn MovetoSelectedTile
  (bind _returnvalue (Game|GetPlayerCharacter 0))
  (bind _selectedtile (Variables|Default|GetselectedTile))
  (bind _returnvalue_2 (Transformation|GetActorRotation _returnvalue))
  (bind (_roll _pitch) (Math|Rotator|BreakRotator _returnvalue_2))
  (if (!= _selectedtile 0)
    (Pawn|SetControlRotation (Math|Rotator|MakeRotator _roll _pitch (.Yaw (Math|Rotator|BreakRotator (Math|Rotator|FindLookatRotation (Transformation|GetActorLocation _returnvalue) (Transformation|GetActorLocation _selectedtile))))))
    (Variables|Default|SetstartLocation (Transformation|GetActorLocation _returnvalue))
    (Variables|Default|SetisMoving true)
    (bind (_fuelcost _foodcost) (CallFunction|CalculateCost "NewEnumerator0" false))
    (CallFunction|AppendEventtoLog (Utilities|String|Append "Moved to " (Variables|/Game/Tiles/A_BasePlayableTile.A_BasePlayableTile_C|GetGameDisplayName (Variables|Default|GetselectedTile)) "(Fuel: " (Utilities|String|ToString(Integer) _fuelcost) ", Food:" (Utilities|String|ToString(Integer) _foodcost) ") 
"))
    (CallFunction|UpdateGameParams _fuelcost _foodcost)
    (CallFunction|MoveCharacter)))

(fn ResetSelection
  (Default|ToggleSelection (Variables|Default|GetselectedTile))
  (Variables|Default|SetselectedTile 0))

(fn SelectTile
  (params (tile :type A%20Base%20Playable%20Tile%20Object%20Reference))
  (if (not (Variables|Default|GetisMoving))
    (if (not (== (Variables|Default|GetselectedTile) tile))
      (Default|ToggleSelection tile)
      (if (!= (Variables|Default|GetselectedTile) 0)
        (Default|ToggleSelection (Variables|Default|GetselectedTile)))
      (Variables|Default|SetselectedTile tile))))

(fn MovetoNextLayer
  (bind _returnvalue (Game|GetPlayerCharacter 0))
  (Transformation|SetActorLocation _returnvalue (Math|Vector|MakeVector (Math|Conversions|ToFloat(Integer) (+ (* (Variables|Default|GetspawnIndex) 100) 50)) 5e+01 (.Z (Math|Vector|BreakVector (Transformation|GetActorLocation _returnvalue)))) false false)
  (Variables|Default|SetselectedTile 0)
  (Variables|Default|SetcurrentTile 0)
  (Variables|Default|SetreadyToMoveOn false)
  (Variables|Default|SetgameCityLayersLeft (- (Variables|Default|GetgameCityLayersLeft) 1))
  (Variables|Default|SetfireEatenTileRows 0)
  (Variables|Default|SetmovesBeforeFireWalk 2)
  (if (Variables|Default|GetisInitialMove)
    (Variables|Default|SetisInitialMove false)
    (else
      (bind (_fuelcost _foodcost) (CallFunction|CalculateCost "NewEnumerator1" false))
      (CallFunction|AppendEventtoLog (Utilities|String|Append "Moved to " "Next Layer (Fuel: " (Utilities|String|ToString(Integer) _fuelcost) ", Food:" (Utilities|String|ToString(Integer) _foodcost) ") 
"))
      (CallFunction|UpdateGameParams _fuelcost _foodcost)))
  (bind _shouldcontinue (CallFunction|VerifyLoseCondition))
  (return _shouldcontinue))

(fn GenerateLevel
  (bind _returnvalue (Math|Random|RandomFloat))
  (bind _shouldcontinue (CallFunction|MovetoNextLayer))
  (if _shouldcontinue
    (CallFunction|ResetLog)
    ;[1 1 1] remove previous tiles
    (bind _outactors (Actor|GetAllActorsOfClass "/Game/Tiles/A_BaseTile.A_BaseTile_C"))
    (for _array_element _outactors
      (Actor|DestroyActor _array_element))
    ;[1 1 1] remove fire tiles from playable area
    (bind _outactors_2 (Actor|GetAllActorsOfClass "/Game/Tiles/A_FireTile.A_FireTile_C"))
    (for _array_element_2 _outactors_2
      (Math|Integer|CompareInt (Variables|/Game/Tiles/A_FireTile.A_FireTile_C|GettileRow _array_element_2)
        (:>
          _)
        (:==
          _))
      (Actor|DestroyActor _array_element_2))
    ;[1 1 1] generate new non last level
    (for _index (range 0 (Variables|Default|GetmaxPlayableRows))
      (for _index_2 (range 0 6)
        (if (|((Index==0)||(index=={0966632F-46A8-0CD3-9C8E-76AE1BB9CC44})) _index)
          (bind _returnvalue_2 (Game|SpawnActorfromClass "/Game/Tiles/A_CityWall.A_CityWall_C" (Math|Transform|MakeTransform (Math|Vector|MakeVector (* _index_2 1e+02) (* _index 1e+02) 0.1)) "Undefined" 0 0))
          (if (== _index (Variables|Default|GetmaxPlayableRows))
            (Variables|/Game/Tiles/A_BasePlayableTile.A_BasePlayableTile_C|SetInLastLine _returnvalue_2 true)
            (Variables|/Game/Tiles/A_BasePlayableTile.A_BasePlayableTile_C|Setindex _returnvalue_2 _index_2))
          (Variables|/Game/Tiles/A_BaseTile.A_BaseTile_C|SettileRow _returnvalue_2 _index)
          (elif (Math|Float|InRange(Float) _returnvalue 0.0 0.6)
            (bind _returnvalue_3 (Game|SpawnActorfromClass "/Game/Tiles/A_Field.A_Field_C" (Math|Transform|MakeTransform (Math|Vector|MakeVector (* _index_2 1e+02) (* _index 1e+02) 0.1)) "Undefined" 0 0))
            (Variables|/Game/Tiles/A_BaseTile.A_BaseTile_C|SettileRow _returnvalue_3 _index)
            (elif (Math|Float|InRange(Float) _returnvalue 0.6 0.75 false)
              (bind _returnvalue_4 (Game|SpawnActorfromClass "/Game/Tiles/A_Forest.A_Forest_C" (Math|Transform|MakeTransform (Math|Vector|MakeVector (* _index_2 1e+02) (* _index 1e+02) 0.1)) "Undefined" 0 0))
              (Variables|/Game/Tiles/A_BasePlayableTile.A_BasePlayableTile_C|SetGameDisplayName _returnvalue_4 (Utilities|String|Append "Forest " (Utilities|String|ToString(Integer) (+ (LocalVariables|GetforestCount) 1))))
              (LocalVariables|SetforestCount (+ (LocalVariables|GetforestCount) 1))
              (Variables|/Game/Tiles/A_BaseTile.A_BaseTile_C|SettileRow _returnvalue_4 _index)
              (elif (Math|Float|InRange(Float) _returnvalue 0.75 0.95 false)
                (bind _returnvalue_5 (Game|SpawnActorfromClass "/Game/Tiles/A_Village.A_Village_C" (Math|Transform|MakeTransform (Math|Vector|MakeVector (* _index_2 1e+02) (* _index 1e+02) 0.1)) "Undefined" 0 0))
                (Variables|/Game/Tiles/A_BasePlayableTile.A_BasePlayableTile_C|SetGameDisplayName _returnvalue_5 (Utilities|String|Append "Village " (Utilities|String|ToString(Integer) (+ (LocalVariables|GetvillageCount) 1))))
                (LocalVariables|SetvillageCount (+ (LocalVariables|GetvillageCount) 1))
                (Variables|/Game/Tiles/A_BaseTile.A_BaseTile_C|SettileRow _returnvalue_5 _index)
                (else
                  (bind _returnvalue_6 (Game|SpawnActorfromClass "/Game/Tiles/A_Pond.A_Pond_C" (Math|Transform|MakeTransform (Math|Vector|MakeVector (* _index_2 1e+02) (* _index 1e+02) 0.1)) "Undefined" 0 0))
                  (Variables|/Game/Tiles/A_BaseTile.A_BaseTile_C|SettileRow _returnvalue_6 _index))))))))))

(fn UpdateStateAfterMoveDidFinished
  (bind _selectedtile (Variables|Default|GetselectedTile))
  (Variables|Default|SetisMoving false)
  (if (Variables|/Game/Tiles/A_BasePlayableTile.A_BasePlayableTile_C|GetInLastLine _selectedtile)
    (Variables|Default|SetreadyToMoveOn true)
    (Variables|Default|SetspawnIndex (Variables|/Game/Tiles/A_BasePlayableTile.A_BasePlayableTile_C|Getindex _selectedtile))
    (else
      (Variables|Default|SetreadyToMoveOn false)
      (Variables|Default|SetspawnIndex 3)))
  (Variables|Default|SetcurrentTile _selectedtile)
  (Math|Integer|CompareInt (Variables|Default|GetmovesBeforeFireWalk)
    (:>
      (bind _output_get (Variables|Default|SetmovesBeforeFireWalk (- (Variables|Default|GetmovesBeforeFireWalk) 1)))
      (CallFunction|AppendEventtoLog (Utilities|String|Append "Fire will start spreading in " (Utilities|String|ToString(Integer) (+ _output_get 1)) " moves" " 
")))
    (:==
      _)
    (:<
      _))
  (bind _shouldcontinue (CallFunction|VerifyLoseCondition))
  (if _shouldcontinue
    (CallFunction|FireEatPlayableAreaifNeeded)))

(fn MoveActor
  (params (Distance :type Float%20%28single-precision%29))
  (bind _returnvalue (Game|GetPlayerCharacter 0))
  (bind _selectedtile (Variables|Default|GetselectedTile))
  (bind _startlocation (Variables|Default|GetstartLocation))
  (bind _returnvalue_2 (Transformation|GetActorLocation _selectedtile))
  (bind (_x _y) (Math|Vector|BreakVector _returnvalue_2))
  (bind _returnvalue_3 (+ _y 5e+01))
  (bind _returnvalue_4 (+ _x 5e+01))
  (Utilities|Casting|CastToA_CityWall _selectedtile
    (:then
      (Transformation|SetActorLocation _returnvalue (Math|Vector|Lerp(Vector) _startlocation (Math|Vector|MakeVector _returnvalue_4 _returnvalue_3 9e+01) Distance) false true))
    (:CastFailed
      (Transformation|SetActorLocation _returnvalue (Math|Vector|Lerp(Vector) _startlocation (Math|Vector|MakeVector _returnvalue_4 _returnvalue_3 9e+01) Distance) false true))))

(fn VerifyLoseCondition
  (Math|Integer|CompareInt (Variables|Default|GetgameHullHP)
    (:>
      (Math|Integer|CompareInt (Variables|Default|GetgameFuel)
        (:>
          (Math|Integer|CompareInt (Variables|Default|GetgameCrewSize)
            (:>
              (Math|Integer|CompareInt (Variables|Default|GetgameFood)
                (:>
                  (bind _shouldcontinue (CallFunction|VerifyWinCondition))
                  (return _shouldcontinue))
                (:==
                  _)
                (:<
                  _)))
            (:==
              _)
            (:<
              _)))
        (:==
          _)
        (:<
          _)))
    (:==
      _)
    (:<
      _))
  (CallFunction|GenerateGameOver)
  (return false))

(fn GenerateGameOver
  (Rendering|SetVisibility (Variables|/Script/Engine.Character|GetCapsuleComponent (Game|GetPlayerCharacter 0)) false true)
  (Viewport|RemoveAllWidgets)
  (bind _returnvalue (UserInterface|CreateWidget "/Game/UI/UI_GameOver.UI_GameOver_C"))
  (UserInterface|Viewport|AddtoViewport _returnvalue 0)
  (bind _outactors (Actor|GetAllActorsOfClass "/Game/Tiles/A_BaseTile.A_BaseTile_C"))
  (for _array_element _outactors
    (Actor|DestroyActor _array_element))
  (for _index (range 0 (Variables|Default|GetmaxPlayableRows))
    (for _index_2 (range 0 6)
      (bind _returnvalue_2 (Game|SpawnActorfromClass "/Game/Tiles/A_FireTile.A_FireTile_C" (Math|Transform|MakeTransform (Math|Vector|MakeVector (* _index_2 1e+02) (* _index 1e+02) 0.1)) "Undefined" 0 0))
      (if (Math|Float|InRange(Float) (Math|Random|RandomFloat) 0.75 1.0)
        (Default|StartParticles _returnvalue_2)))))

(fn VerifyWinCondition
  (Math|Integer|CompareInt (Variables|Default|GetgameCityLayersLeft)
    (:>
      (return true))
    (:==
      _)
    (:<
      _))
  (CallFunction|GenerateWinScreen)
  (return false))

(fn GenerateWinScreen
  (bind _returnvalue (Math|Random|RandomFloat))
  ;[1 1 1] win widget
  (Viewport|RemoveAllWidgets)
  (bind _returnvalue_2 (UserInterface|CreateWidget "/Game/UI/UI_Win.UI_Win_C"))
  (UserInterface|Viewport|AddtoViewport _returnvalue_2 0)
  ;[1 1 1] destroy fire tiles
  (bind _outactors (Actor|GetAllActorsOfClass "/Game/Tiles/A_FireTile.A_FireTile_C"))
  (for _array_element _outactors
    (Default|StopParticles _array_element)
    (Actor|DestroyActor _array_element))
  ;[1 1 1] remove previous tiles
  (bind _outactors_2 (Actor|GetAllActorsOfClass "/Game/Tiles/A_BaseTile.A_BaseTile_C"))
  (for _array_element_2 _outactors_2
    (Actor|DestroyActor _array_element_2))
  ;[1 1 1] generate ponds instead of fire
  (for _index (range 0 3)
    (for _index_2 (range 0 6)
      (Game|SpawnActorfromClass "/Game/Tiles/A_Pond.A_Pond_C" (Math|Transform|MakeTransform (Math|Vector|MakeVector (* _index_2 1e+02) (* (+ _index 1) -1e+02) 0.1)) "Undefined" 0 0)))
  ;[1 1 1] generate new last level
  (for _index_3 (range 0 (Variables|Default|GetmaxPlayableRows))
    (for _index_4 (range 0 6)
      (if (|(Index==0) _index_3)
        (bind _returnvalue_3 (Game|SpawnActorfromClass "/Game/Tiles/A_CityWall.A_CityWall_C" (Math|Transform|MakeTransform (Math|Vector|MakeVector (* _index_4 1e+02) (* _index_3 1e+02) 0.1)) "Undefined" 0 0))
        (if (== _index_3 8)
          (Variables|/Game/Tiles/A_BasePlayableTile.A_BasePlayableTile_C|SetInLastLine _returnvalue_3 true)
          (Variables|/Game/Tiles/A_BasePlayableTile.A_BasePlayableTile_C|Setindex _returnvalue_3 _index_4))
        (elif (Math|Float|InRange(Float) _returnvalue 0.0 0.6)
          (Game|SpawnActorfromClass "/Game/Tiles/A_Village.A_Village_C" (Math|Transform|MakeTransform (Math|Vector|MakeVector (* _index_4 1e+02) (* _index_3 1e+02) 0.1)) "Undefined" 0 0)
          (elif (Math|Float|InRange(Float) _returnvalue 0.6 0.75 false)
            (Game|SpawnActorfromClass "/Game/Tiles/A_Forest.A_Forest_C" (Math|Transform|MakeTransform (Math|Vector|MakeVector (* _index_4 1e+02) (* _index_3 1e+02) 0.1)) "Undefined" 0 0)
            (elif (Math|Float|InRange(Float) _returnvalue 0.75 0.95 false)
              (Game|SpawnActorfromClass "/Game/Tiles/A_Field.A_Field_C" (Math|Transform|MakeTransform (Math|Vector|MakeVector (* _index_4 1e+02) (* _index_3 1e+02) 0.1)) "Undefined" 0 0)
              (else
                (Game|SpawnActorfromClass "/Game/Tiles/A_Pond.A_Pond_C" (Math|Transform|MakeTransform (Math|Vector|MakeVector (* _index_4 1e+02) (* _index_3 1e+02) 0.1)) "Undefined" 0 0)))))))))

(fn UpdateMoveProgressifNeeded
  (params (Delta :type Float%20%28single-precision%29))
  (bind _selectedtile (Variables|Default|GetselectedTile))
  (bind _startlocation (Variables|Default|GetstartLocation))
  (bind _returnvalue (Transformation|GetActorLocation _selectedtile))
  (if (Variables|Default|GetisMoving)
    (if (Math|Vector|NotEqual(Vector) _returnvalue _startlocation 0.0001)
      (bind _output_get (Variables|Default|SetmoveProgress (+ (/ (* Delta (Variables|Default|GetgameVehicleSpeed)) (Math|Vector|Distance(Vector) _startlocation _returnvalue)) (Variables|Default|GetmoveProgress))))
      (CallFunction|MoveActor _output_get)
      (if (>= (Variables|Default|GetmoveProgress) 1.0)
        (CallFunction|UpdateStateAfterMoveDidFinished :!label _label))
      (else
        (Variables|Default|SetmoveProgress 1.0)
        (goto _label)))))

(fn CalculateCost
  (params (purpose :type CostPurpose%20Enum :default "NewEnumerator0") (shouldTryRandomEvent :type Boolean))
  (bind _returnvalue (Game|GetPlayerCharacter 0))
  (bind _returnvalue_2 (Math|Random|RandomFloat))
  (bind _selectedtile (Variables|Default|GetselectedTile))
  (bind _gamecrewsize (Variables|Default|GetgameCrewSize))
  (bind _selectedtile_2 (Variables|Default|GetselectedTile))
  (bind _currenttile (Variables|Default|GetcurrentTile))
  (bind _returnvalue_3 (Transformation|GetActorLocation _currenttile))
  (bind _returnvalue_4 (Transformation|GetActorLocation _returnvalue))
  (bind _returnvalue_5 (Transformation|GetActorLocation _selectedtile_2))
  (bind _returnvalue_6 (Math|Float|InRange(Float) _returnvalue_2 0.0 0.8))
  (bind _returnvalue_7 (Math|Vector|Distance(Vector) _returnvalue_3 _returnvalue_5))
  (bind _returnvalue_8 (Math|Vector|Distance(Vector) _returnvalue_4 _returnvalue_5))
  (switch Utilities|FlowControl|Switch|SwitchonCostPurpose purpose
    (:NewEnumerator0
      (if (!= _selectedtile_2 0)
        (if (!= _currenttile 0)
          (Math|Float|CompareFloat _returnvalue_7 2e+02
            (:>
              (Math|Float|CompareFloat _returnvalue_7 4e+02
                (:>
                  (Math|Float|CompareFloat _returnvalue_7 6e+02
                    (:>
                      (Math|Float|CompareFloat _returnvalue_8 7e+02
                        (:>
                          (return -25 (* _gamecrewsize -5)))
                        (:==
                          _)
                        (:<
                          _))
                      (return -20 (* _gamecrewsize -4)))
                    (:==
                      _)
                    (:<
                      _))
                  (return -15 (* _gamecrewsize -3)))
                (:==
                  _)
                (:<
                  _))
              (return -10 (* _gamecrewsize -2)))
            (:==
              _)
            (:<
              _))
          (else
            (Math|Float|CompareFloat _returnvalue_8 2e+02
              (:>
                (Math|Float|CompareFloat _returnvalue_8 4e+02
                  (:>
                    (Math|Float|CompareFloat _returnvalue_8 6e+02
                      (:>
                        (Math|Float|CompareFloat _returnvalue_8 7e+02
                          (:>
                            (return -25 (* _gamecrewsize -5)))
                          (:==
                            _)
                          (:<
                            _))
                        (return -20 (* _gamecrewsize -4)))
                      (:==
                        _)
                      (:<
                        _))
                    (return -15 (* _gamecrewsize -3)))
                  (:==
                    _)
                  (:<
                    _))
                (return -10 (* _gamecrewsize -2)))
              (:==
                _)
              (:<
                _))))
        (return -5 (* _gamecrewsize -1))
        (else
          _)))
    (:NewEnumerator1
      (return -20 -20))
    (:NewEnumerator2
      (if (!= _selectedtile 0)
        (Utilities|Casting|CastToA_Forest _selectedtile
          (:then
            (if shouldTryRandomEvent
              (if _returnvalue_6
                _
                (else
                  (CallFunction|AppendEventtoLog (Utilities|String|MakeLiteralString "In the forest you found wolfs and run away 
"))
                  (CallFunction|AppendEventtoNotification)
                  ;[1 1 1] haunted forest
                  (return 0 20))))
            ;[1 1 1] forest
            (return 0 40))
          (:CastFailed
            (if shouldTryRandomEvent
              (if _returnvalue_6
                _
                (else
                  (switch int (Math|Random|RandomIntegerinRange 0 1)
                    (:Default
                      (CallFunction|AppendEventtoLog (Utilities|String|MakeLiteralString "You find an plundered village 
") :!label _label)
                      (CallFunction|AppendEventtoNotification))
                    (:0
                      (goto _label))
                    (:1
                      (CallFunction|AppendEventtoLog (Utilities|String|MakeLiteralString "Village fanatics tried to sabotage your ship 
"))
                      (CallFunction|AppendEventtoNotification)))
                  ;[1 1 1] Empty Village
                  (return 15 5))))
            ;[1 1 1] Village
            (return 30 10)))
        (else
          _))))
  ;[1 1 1] Not expected
  (return 0 0))

(fn UpdateGameParams
  (params (Fuel :type Integer) (Food :type Integer) (Hull :type Integer))
  ;[1 1 1] Fuel
  (Math|Integer|CompareInt (+ (Variables|Default|GetgameFuel) Fuel)
    (:>
      (Math|Integer|CompareInt (+ (Variables|Default|GetgameFuel) Fuel) 100
        (:>
          (Variables|Default|SetgameFuel 100))
        (:==
          (Variables|Default|SetgameFuel (+ (Variables|Default|GetgameFuel) Fuel) :!label _label))
        (:<
          (goto _label))))
    (:==
      (Variables|Default|SetgameFuel 0 :!label _label_2))
    (:<
      (goto _label_2)))
  ;[1 1 1] Food
  (Math|Integer|CompareInt (+ (Variables|Default|GetgameFood) Food)
    (:>
      (Math|Integer|CompareInt (+ (Variables|Default|GetgameFood) Food) 200
        (:>
          (Variables|Default|SetgameFood 200))
        (:==
          (Variables|Default|SetgameFood (+ (Variables|Default|GetgameFood) Food) :!label _label_3))
        (:<
          (goto _label_3))))
    (:==
      (Variables|Default|SetgameFood 0 :!label _label_4))
    (:<
      (goto _label_4)))
  ;[1 1 1] Hull
  (Math|Integer|CompareInt (+ (Variables|Default|GetgameHullHP) Hull)
    (:>
      (Math|Integer|CompareInt (+ (Variables|Default|GetgameHullHP) Hull) 100
        (:>
          (Variables|Default|SetgameHullHP 100))
        (:==
          (Variables|Default|SetgameHullHP (+ (Variables|Default|GetgameHullHP) Hull) :!label _label_5))
        (:<
          (goto _label_5))))
    (:==
      (Variables|Default|SetgameHullHP 0 :!label _label_6))
    (:<
      (goto _label_6))))

(fn Interact
  (bind _currenttile (Variables|Default|GetcurrentTile))
  (bind _currenttile_2 (Variables|Default|GetcurrentTile))
  (bind _currenttile_3 (Variables|Default|GetcurrentTile))
  (bind _gamedisplayname (Variables|/Game/Tiles/A_BasePlayableTile.A_BasePlayableTile_C|GetGameDisplayName _currenttile_2))
  (if (!= _currenttile_3 0)
    (if (Variables|/Game/Tiles/A_BasePlayableTile.A_BasePlayableTile_C|GetcouldInteract _currenttile_3)
      (bind (_fuelcost _foodcost) (CallFunction|CalculateCost "NewEnumerator2" true))
      (Math|Integer|CompareInt _fuelcost
        (:>
          (CallFunction|AppendEventtoLog (Utilities|String|Append "Interact with " _gamedisplayname "(Fuel: " (Utilities|String|ToString(Integer) _fuelcost) ", Food:" (Utilities|String|ToString(Integer) _foodcost) ") 
") :!label _label))
        (:==
          (CallFunction|AppendEventtoLog (Utilities|String|Append "Interact with " _gamedisplayname " (Food:" (Utilities|String|ToString(Integer) _foodcost) ") 
")))
        (:<
          (goto _label)))
      (CallFunction|UpdateGameParams _fuelcost _foodcost)
      (Variables|/Game/Tiles/A_BasePlayableTile.A_BasePlayableTile_C|SetcouldInteract _currenttile false)
      (Default|SetInactive _currenttile))))

(fn AppendEventtoLog
  (params (NewParam :type String))
  (bind _foundwidgets (Widget|GetAllWidgetsOfClass "/Game/UI/UI_InGame.UI_InGame_C" true))
  (Rendering|Components|TextRender|SetText (Variables|/Game/UI/UI_InGame.UI_InGame_C|GetLogTextBox (Utilities|Array|Get(acopy) _foundwidgets)) (Utilities|Text|ToText(String) (Utilities|String|Append (Utilities|String|ToString(Text) (Class|MultiLineEditableTextBox|GetText (Variables|/Game/UI/UI_InGame.UI_InGame_C|GetLogTextBox (Utilities|Array|Get(acopy) _foundwidgets)))) NewParam)))
  (Class|ScrollBox|ScrolltoEnd (Variables|/Game/UI/UI_InGame.UI_InGame_C|GetScrollBox_165 (Utilities|Array|Get(acopy) _foundwidgets))))

(fn FireEatPlayableAreaifNeeded
  (Math|Integer|CompareInt (Variables|Default|GetmovesBeforeFireWalk)
    (:==
      _)
    (:<
      _))
  (bind _outactors (Actor|GetAllActorsOfClass "/Game/Tiles/A_BaseTile.A_BaseTile_C"))
  (bind _array_element (Utilities|Array|ForEachLoopwithBreak _outactors :!label _label)
    (:LoopBody
      (Math|Integer|CompareInt (Variables|/Game/Tiles/A_BaseTile.A_BaseTile_C|GettileRow _array_element) (Variables|Default|GetfireEatenTileRows)
        (:==
          _)
        (:<
          _))
      (bind _asmy_player_controller (Utilities|Casting|CastToMyPlayerController (Game|GetPlayerController 0)))
      (if (== (Variables|MyPlayerController_C|GetcurrentTile _asmy_player_controller) _array_element)
        (LocalVariables|SetisGameOver true)
        (goto _label Break)
        (else
          (Actor|DestroyActor _array_element))))
    (:Completed
      (if (LocalVariables|GetisGameOver)
        (CallFunction|GenerateGameOver)
        (else
          (CallFunction|GenerateFireTiles (Variables|Default|GetfireEatenTileRows) (Variables|Default|GetfireEatenTileRows))
          (Variables|Default|SetfireEatenTileRows (+ (Variables|Default|GetfireEatenTileRows) 1)))))))

(fn GenerateFireTiles
  (params (startIndex :type Integer) (endIndex :type Integer))
  (for _index (range startIndex endIndex)
    (for _index_2 (range 0 6)
      (bind _returnvalue (Game|SpawnActorfromClass "/Game/Tiles/A_FireTile.A_FireTile_C" (Math|Transform|MakeTransform (Math|Vector|MakeVector (* _index_2 1e+02) (* _index 1e+02) 0.1)) "Undefined" 0 0))
      (if (Math|Float|InRange(Float) (Math|Random|RandomFloat) 0.5 1.0)
        (Default|StartParticles _returnvalue))
      (Variables|/Game/Tiles/A_FireTile.A_FireTile_C|SettileRow _returnvalue _index))))

(fn ResetLog
  (bind _foundwidgets (Widget|GetAllWidgetsOfClass "/Game/UI/UI_InGame.UI_InGame_C" true))
  (Rendering|Components|TextRender|SetText (Variables|/Game/UI/UI_InGame.UI_InGame_C|GetLogTextBox (Utilities|Array|Get(acopy) _foundwidgets)) (Utilities|Text|ToText(String) "")))

(fn AppendEventtoNotification
  (params (NewParam :type String))
  (Utilities|Array|Add (Variables|Default|Getnotifications) "Sabotage happened!")
  (bind _foundwidgets (Widget|GetAllWidgetsOfClass "/Game/UI/UI_InGame.UI_InGame_C" true))
  (Default|UpdateNotifications (Utilities|Array|Get(acopy) _foundwidgets))
  (Utilities|Time|SetTimerbyFunctionName 0 "RemoveNotificationItem" 2.0))

(fn RemoveNotificationItem
  (bind _notifications (Variables|Default|Getnotifications))
  (Math|Integer|CompareInt (Utilities|Array|Length _notifications)
    (:>
      (Utilities|Array|RemoveIndex _notifications)
      (bind _foundwidgets (Widget|GetAllWidgetsOfClass "/Game/UI/UI_InGame.UI_InGame_C" true))
      (Default|UpdateNotifications (Utilities|Array|Get(acopy) _foundwidgets)))))